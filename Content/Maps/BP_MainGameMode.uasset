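; Main game mode for a coin-collecting game, handling score, background music, UI and game flow.
; BeginPlay creates the main UI and plays a music track, with both Sequence branches wired into the same AddToViewport.
; GetCoin adds points to Score by bronze, silver or gold coin type.
; GameOver shows its widget with cursor and UI-only input; Restart reopens the MainGame level and sets game-only input.
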(event Custom|GetCoin
  (params (CoinType :type ENUM_CoinType%20Enum :default "NewEnumerator0"))
  ;[1 1 1] 코인 점수화
  (switch Utilities|FlowControl|Switch|SwitchonENUM_CoinType CoinType
    (:NewEnumerator0
      (Variables|Default|SetScore (+ (Variables|Default|GetScore) 1)))
    (:NewEnumerator1
      (Variables|Default|SetScore (+ (Variables|Default|GetScore) 5)))
    (:NewEnumerator2
      (Variables|Default|SetScore (+ (Variables|Default|GetScore) 10)))))

(event Custom|GameOver
  (bind _returnvalue (Game|GetPlayerController 0))
  ;[1 1 1] 게임오버 UI
  (bind _returnvalue_2 (UserInterface|CreateWidget "/Game/UMG/UMG_GameOver.UMG_GameOver_C"))
  (UserInterface|Viewport|AddtoViewport _returnvalue_2 0)
  (Variables|/Script/Engine.PlayerController|SetbShowMouseCursor _returnvalue true)
  (Input|SetInputModeUIOnly _returnvalue _returnvalue_2 "DoNotLock" false))

(event Custom|Restart
  ;[1 1 1] 레벨 재시작
  (Game|OpenLevel(byName) "MainGame")
  (Input|SetInputModeGameOnly (Game|GetPlayerController 0) false))

(event EventBeginPlay
  (Utilities|FlowControl|Sequence
    (:then_0
      (bind _returnvalue (UserInterface|CreateWidget "/Game/UMG/UMG_MainUI.UMG_MainUI_C")))
    (:then_1
      (Audio|PlaySound2D "/Game/Sounds/Lazy-Laura-Quincas-Moreira.Lazy-Laura-Quincas-Moreira" 0.5 1.0 0.0 0 0)))
  (UserInterface|Viewport|AddtoViewport _returnvalue 0))

(event EventTick
  (params (DeltaSeconds :type Float%20%28single-precision%29)))

(fn ConstructionScript)
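; BP_MovingPlatformfloor is a trigger floor that tells a MovingPlatform when the third-person player character enters or leaves its Box volume.
; Box begin overlap calls InCollision on MovingPlatform and sets IsActive; end overlap calls OutCollision and clears it.
; The IsActive flag blocks repeated enter or exit calls, and a cast to BP_ThirdPersonCharacter filters out other actors.
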(event OnComponentBeginOverlap(Box)
  (params (OverlappedComponent :type Primitive%20Component%20Object%20Reference) (OtherActor :type Actor%20Object%20Reference) (OtherComp :type Primitive%20Component%20Object%20Reference) (OtherBodyIndex :type Integer) (bFromSweep :type Boolean) (SweepResult :type Hit%20Result%20Structure%20%28by%20ref%29))
  (if (not (Variables|Default|GetIsActive))
    (Utilities|Casting|CastToBP_ThirdPersonCharacter OtherActor)
    (Utilities|FlowControl|Sequence
      (:then_0
        (Default|InCollision (Variables|Default|GetMovingPlatform)))
      (:then_1
        (Variables|Default|SetIsActive true)))))

(event OnComponentEndOverlap(Box)
  (params (OverlappedComponent :type Primitive%20Component%20Object%20Reference) (OtherActor :type Actor%20Object%20Reference) (OtherComp :type Primitive%20Component%20Object%20Reference) (OtherBodyIndex :type Integer))
  (if (Variables|Default|GetIsActive)
    (Utilities|Casting|CastToBP_ThirdPersonCharacter OtherActor)
    (Utilities|FlowControl|Sequence
      (:then_0
        (Default|OutCollision (Variables|Default|GetMovingPlatform)))
      (:then_1
        (Variables|Default|SetIsActive false)))))

(event EventBeginPlay)

(event Collision|EventActorBeginOverlap
  (params (OtherActor :type Actor%20Object%20Reference)))

(event EventTick
  (params (DeltaSeconds :type Float%20%28single-precision%29)))

(fn ConstructionScript)